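; Blueprint for the Poron enemy character, linking its overhead health bar widget and attack range trigger to enemy logic.
; SetUILV and DamageHealth cast the HealthBar component's widget to EHPBar, then write the level text and set the bar's percent directly from the passed value.
; Atkrange begin and end overlaps forward to RangeOverlap and EndRangeOverlap, whose logic lives outside these graphs.
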(event `self.SetUILV`
  (bind _asehpbar (cast `/Game/UI/EHPBar` (`WidgetComponent.GetUserWidgetObject` (`self.HealthBar`))))
  (`TextBlock.SetText` (`/Game/UI/EHPBar.LvText` _asehpbar) (`KismetTextLibrary.Conv_IntToText` (`self.Lv`) false true 1 10)))

(event `self.DamageHealth`
  (params (Dmg :type "Float (single-precision) (by ref)"))
  (bind _asehpbar (cast `/Game/UI/EHPBar` (`WidgetComponent.GetUserWidgetObject` (`self.HealthBar`))))
  (`ProgressBar.SetPercent` (`/Game/UI/EHPBar.EHealthbarWidg` _asehpbar) Dmg))

(event `self.Atkrange.OnComponentBeginOverlap`
  (params (OverlappedComponent :type "PrimitiveComponent Object Reference") (OtherActor :type "Actor Object Reference") (OtherComp :type "PrimitiveComponent Object Reference") (OtherBodyIndex :type Integer) (bFromSweep :type Boolean) (SweepResult :type "HitResult Structure (by ref)"))
  (`self.RangeOverlap` OtherActor))

(event `self.Atkrange.OnComponentEndOverlap`
  (params (OverlappedComponent :type "PrimitiveComponent Object Reference") (OtherActor :type "Actor Object Reference") (OtherComp :type "PrimitiveComponent Object Reference") (OtherBodyIndex :type Integer))
  (`self.endRangeOverlap`))

(fn `UserConstructionScript`)