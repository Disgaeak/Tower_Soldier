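; Sentinel AI controller that drives a player-side sentinel, targeting actors tagged Enemy.
; On BeginPlay it sets up the PlayerSentinel_BB blackboard, runs the PlayerSentinelAI behavior tree and caches the blackboard component.
; AI perception updates write a successfully sensed enemy to the Target key only while that key is empty, so this controller never replaces or clears an acquired target.
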(event `self.ReceiveBeginPlay`
  (bind _blackboardcomponent (`self.UseBlackboard` "/Game/Characters/Players/AI/PlayerSentinel_BB.PlayerSentinel_BB"))
  (`self.RunBehaviorTree` "/Game/Characters/Players/AI/PlayerSentinelAI.PlayerSentinelAI")
  (set `self.BBRef` _blackboardcomponent))

(event `self.AIPerception.OnTargetPerceptionUpdated`
  (params (Actor :type "Actor Object Reference") (Stimulus :type "AIStimulus Structure"))
  (bind _bbref (`self.BBRef`))
  (bind _target (`self.Target`))
  (if (== (`BlackboardComponent.GetValueAsObject` (`self.BBRef`) (`self.Target`)) null)
    (if (and (`self.ActorHasTag` Actor "Enemy") (`.bSuccessfullySensed` (break `AIStimulus` Stimulus)))
      (`BlackboardComponent.SetValueAsObject` _bbref _target Actor)
      (else
        (`BlackboardComponent.SetValueAsObject` _bbref _target null)))))

(fn `UserConstructionScript`)