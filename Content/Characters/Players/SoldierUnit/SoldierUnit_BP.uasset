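; SoldierUnit_BP is a player soldier unit with an overhead health bar widget and an attack range trigger.
; UIChange and DamageHealth cast the HealthBar widget to HPBar to set the level number text and the bar percent.
; Overlaps entering Atkrange are passed unfiltered to RangeOverlap, while only actors tagged Enemy leaving it call EndAtkTime.
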(event `self.UIChange`
  (bind _ashpbar (cast `/Game/UI/HPBar` (`WidgetComponent.GetUserWidgetObject` (`self.HealthBar`))))
  (`TextBlock.SetText` (`/Game/UI/HPBar.LvNumWidg` _ashpbar) (`KismetTextLibrary.Conv_IntToText` (`self.Lv`) false true 1 10)))

(event `self.DamageHealth`
  (params (Dmg :type "Float (single-precision) (by ref)"))
  (bind _ashpbar (cast `/Game/UI/HPBar` (`WidgetComponent.GetUserWidgetObject` (`self.HealthBar`))))
  (`ProgressBar.SetPercent` (`/Game/UI/HPBar.HealthBarWidg` _ashpbar) Dmg))

(event `self.Atkrange.OnComponentBeginOverlap`
  (params (OverlappedComponent :type "PrimitiveComponent Object Reference") (OtherActor :type "Actor Object Reference") (OtherComp :type "PrimitiveComponent Object Reference") (OtherBodyIndex :type Integer) (bFromSweep :type Boolean) (SweepResult :type "HitResult Structure (by ref)"))
  (`self.RangeOverlap` OtherActor))

(event `self.Atkrange.OnComponentEndOverlap`
  (params (OverlappedComponent :type "PrimitiveComponent Object Reference") (OtherActor :type "Actor Object Reference") (OtherComp :type "PrimitiveComponent Object Reference") (OtherBodyIndex :type Integer))
  (if (`self.ActorHasTag` OtherActor "Enemy")
    (`self.EndAtkTime`)))

(fn `UserConstructionScript`)