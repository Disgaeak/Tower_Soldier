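; Stage 1-1 level tile for a tower defence game, with trigger volumes for the stage's gates and endpoint.
; Enemies reaching the endpoint damage the town by their level and job, are destroyed, and prompt the child spawner to recheck its enemy array.
; Allies touching the end gate are destroyed.
; The first enemy through the story gate spawns the Klaine sentinel AI near a target point and flags the game mode event.
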(event `self.ReceiveBeginPlay`
  (bind _astower_defence_game_mode (cast `TowerDefenceGameMode` (`GameplayStatics.GetGameMode`)))
  (set `self.GMRef` _astower_defence_game_mode))

(event `self.EndGate.OnComponentBeginOverlap`
  (params (OverlappedComponent :type "PrimitiveComponent Object Reference") (OtherActor :type "Actor Object Reference") (OtherComp :type "PrimitiveComponent Object Reference") (OtherBodyIndex :type Integer) (bFromSweep :type Boolean) (SweepResult :type "HitResult Structure (by ref)"))
  (if (`self.ActorHasTag` OtherActor "Ally")
    (`self.K2_DestroyActor` OtherActor)))

(event `self.Endpoint.OnComponentBeginOverlap`
  (params (OverlappedComponent :type "PrimitiveComponent Object Reference") (OtherActor :type "Actor Object Reference") (OtherComp :type "PrimitiveComponent Object Reference") (OtherBodyIndex :type Integer) (bFromSweep :type Boolean) (SweepResult :type "HitResult Structure (by ref)"))
  (if (`self.ActorHasTag` OtherActor "Enemy")
    (bind _asenemy_base (cast `EnemyBase` OtherActor))
    (bind (_lvl _ahp _amaxhp _aatk _adef _axp _amaxxp _jobnum) (`EnemyBase.GetAllStats` _asenemy_base))
    (`TowerDefenceGameMode.AttackTown` (`self.GMRef`) _lvl _jobnum)
    (`self.K2_DestroyActor` _asenemy_base)
    (bind _asenemy_spawner_bp (cast `/Game/System/EnemySpawner_BP` (`ChildActorComponent.ChildActor` (`self.Spawn`))))
    (`EnemySpawner.CheckEArray` _asenemy_spawner_bp)))

(event `self.StoryGate1.OnComponentBeginOverlap`
  (params (OverlappedComponent :type "PrimitiveComponent Object Reference") (OtherActor :type "Actor Object Reference") (OtherComp :type "PrimitiveComponent Object Reference") (OtherBodyIndex :type Integer) (bFromSweep :type Boolean) (SweepResult :type "HitResult Structure (by ref)"))
  (if (and (== (`|GetArrayItem` (`TowerDefenceGameMode.Events` (`self.GMRef`))) false) (`self.ActorHasTag` OtherActor "Enemy"))
    (`AIBlueprintHelperLibrary.SpawnAIFromClass` "/Game/Characters/Players/Klaine/Klaine_BP.Klaine_BP_C" "/Game/Characters/Players/AI/PlayerSentinelAI.PlayerSentinelAI" (`KismetMathLibrary.MakeVector` (.x (`SceneComponent.K2_GetComponentLocation` (`self.Target`))) (- (.y (`SceneComponent.K2_GetComponentLocation` (`self.Target`))) 200.0) (.z (`SceneComponent.K2_GetComponentLocation` (`self.Target`)))))
    (`KismetArrayLibrary.Array_Set` (`TowerDefenceGameMode.Events` (`self.GMRef`)) 0 true)))

(fn `UserConstructionScript`)