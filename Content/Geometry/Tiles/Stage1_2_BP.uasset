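; Stage 1-2 tile Blueprint for a tower defence level, handling its trigger volumes.
; Enemies reaching the end goal attack the town through the game mode using their level and job, are destroyed, then prompt the child-actor spawner to check its enemy array.
; Three end gates destroy any overlapping allies.
; An ally entering the extra map trigger sets an event flag on the game mode.
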(event `self.ReceiveBeginPlay`
  (bind _astower_defence_game_mode (cast `TowerDefenceGameMode` (`GameplayStatics.GetGameMode`)))
  (set `self.GMRef` _astower_defence_game_mode))

(event `self.EndGate.OnComponentBeginOverlap`
  (params (OverlappedComponent :type "PrimitiveComponent Object Reference") (OtherActor :type "Actor Object Reference") (OtherComp :type "PrimitiveComponent Object Reference") (OtherBodyIndex :type Integer) (bFromSweep :type Boolean) (SweepResult :type "HitResult Structure (by ref)"))
  (`self.CheckOverlap` OtherActor))

(event `self.EndGate1.OnComponentBeginOverlap`
  (params (OverlappedComponent :type "PrimitiveComponent Object Reference") (OtherActor :type "Actor Object Reference") (OtherComp :type "PrimitiveComponent Object Reference") (OtherBodyIndex :type Integer) (bFromSweep :type Boolean) (SweepResult :type "HitResult Structure (by ref)"))
  (`self.CheckOverlap` OtherActor))

(event `self.EndGate2.OnComponentBeginOverlap`
  (params (OverlappedComponent :type "PrimitiveComponent Object Reference") (OtherActor :type "Actor Object Reference") (OtherComp :type "PrimitiveComponent Object Reference") (OtherBodyIndex :type Integer) (bFromSweep :type Boolean) (SweepResult :type "HitResult Structure (by ref)"))
  (`self.CheckOverlap` OtherActor))

(event `self.EndGoal.OnComponentBeginOverlap`
  (params (OverlappedComponent :type "PrimitiveComponent Object Reference") (OtherActor :type "Actor Object Reference") (OtherComp :type "PrimitiveComponent Object Reference") (OtherBodyIndex :type Integer) (bFromSweep :type Boolean) (SweepResult :type "HitResult Structure (by ref)"))
  (if (`self.ActorHasTag` OtherActor "Enemy")
    (bind _asenemy_base (cast `EnemyBase` OtherActor))
    (bind (_lvl _ahp _amaxhp _aatk _adef _axp _amaxxp _jobnum) (`EnemyBase.GetAllStats` _asenemy_base))
    (`TowerDefenceGameMode.AttackTown` (`self.GMRef`) _lvl _jobnum)
    (`self.K2_DestroyActor` _asenemy_base)
    (bind _asenemy_spawner_bp (cast `/Game/System/EnemySpawner_BP` (`ChildActorComponent.ChildActor` (`self.Spawn`))))
    (`EnemySpawner.CheckEArray` _asenemy_spawner_bp)))

(event `self.ExtraMap.OnComponentBeginOverlap`
  (params (OverlappedComponent :type "PrimitiveComponent Object Reference") (OtherActor :type "Actor Object Reference") (OtherComp :type "PrimitiveComponent Object Reference") (OtherBodyIndex :type Integer) (bFromSweep :type Boolean) (SweepResult :type "HitResult Structure (by ref)"))
  (if (`self.ActorHasTag` OtherActor "Ally")
    (`KismetArrayLibrary.Array_Set` (`TowerDefenceGameMode.Events` (`self.GMRef`)) 1 true)))

(fn `CheckOverlap`
  (params (Actor :type "Actor Object Reference"))
  (if (`self.ActorHasTag` Actor "Ally")
    (`self.K2_DestroyActor` Actor)))

(fn `UserConstructionScript`)