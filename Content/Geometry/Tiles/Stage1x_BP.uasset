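; Stage tile actor for a tower defence game that handles enemies reaching the town goal.
; On BeginPlay it caches the TowerDefenceGameMode.
; When an Enemy-tagged actor overlaps EndGoal, it passes the enemy's level and job from GetAllStats to the game mode's AttackTown and destroys the enemy.
; It then has the child-actor EnemySpawner_BP recheck its enemy array via CheckEArray.
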(event `self.ReceiveBeginPlay`
  (bind _astower_defence_game_mode (cast `TowerDefenceGameMode` (`GameplayStatics.GetGameMode`)))
  (set `self.GMRef` _astower_defence_game_mode))

(event `self.EndGoal.OnComponentBeginOverlap`
  (params (OverlappedComponent :type "PrimitiveComponent Object Reference") (OtherActor :type "Actor Object Reference") (OtherComp :type "PrimitiveComponent Object Reference") (OtherBodyIndex :type Integer) (bFromSweep :type Boolean) (SweepResult :type "HitResult Structure (by ref)"))
  (if (`self.ActorHasTag` OtherActor "Enemy")
    (bind _asenemy_base (cast `EnemyBase` OtherActor))
    (bind (_lvl _ahp _amaxhp _aatk _adef _axp _amaxxp _jobnum) (`EnemyBase.GetAllStats` _asenemy_base))
    (`TowerDefenceGameMode.AttackTown` (`self.GMRef`) _lvl _jobnum)
    (`self.K2_DestroyActor` OtherActor)
    (bind _asenemy_spawner_bp (cast `/Game/System/EnemySpawner_BP` (`ChildActorComponent.ChildActor` (`self.SPawn`))))
    (`EnemySpawner.CheckEArray` _asenemy_spawner_bp)))

(fn `UserConstructionScript`)